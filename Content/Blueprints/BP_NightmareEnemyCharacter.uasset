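; BP_NightmareEnemyCharacter is an enemy character with health that can attack the first-person player.
; Hits from a jump boost projectile destroy that projectile and apply fixed damage, destroying the enemy when health runs out.
; AttackPlayer scans AttackCollider overlaps and calls TakeDamage on any FirstPersonCharacter, passing the enemy's control-rotation forward vector rather than a damage amount.
; Nothing in this graph calls AttackPlayer.
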(event `self.ReceiveHit`
  (params (MyComp :type "PrimitiveComponent Object Reference") (Other :type "Actor Object Reference") (OtherComp :type "PrimitiveComponent Object Reference") (bSelfMoved :type Boolean) (HitLocation :type "Vector Structure") (HitNormal :type "Vector Structure") (NormalImpulse :type "Vector Structure") (Hit :type "HitResult Structure (by ref)"))
  (`|ExecutionSequence`
    (:`then_1`
      (bind _asbp_jump_boost_projectile (cast `/Game/FirstPersonCPP/Blueprints/BP_JumpBoostProjectile` Other))
      (`self.TakeDamage` 50)
      (`self.K2_DestroyActor` _asbp_jump_boost_projectile))))

(fn `AttackPlayer`
  (for _array_element (`PrimitiveComponent.GetOverlappingActors` (`self.AttackCollider`) null)
    (bind _asfirst_person_character (cast `/Game/FirstPersonCPP/Blueprints/FirstPersonCharacter` _array_element))
    (`/Game/FirstPersonCPP/Blueprints/FirstPersonCharacter.TakeDamage` _asfirst_person_character (`KismetMathLibrary.GetForwardVector` (`self.GetControlRotation`)))))

(fn `TakeDamage`
  (params (DamageAmount :type Integer))
  (bind _output_get (set `self.Health` (- (`self.Health`) DamageAmount)))
  (if (<= _output_get 0)
    (set `self.Health` 0)
    (`self.K2_DestroyActor`)))

(fn `UserConstructionScript`)